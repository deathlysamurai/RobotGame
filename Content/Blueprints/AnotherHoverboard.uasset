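; Player-controlled hoverboard driven by a physics-simulated sphere, with a mouse-rotated camera boom.
; Each tick the actor follows the sphere, which is held yaw-only, and four socket traces tilt the board to the surface or ease it level when ungrounded.
; WASD sets target speeds, reached through force and torque proportional to the speed error, even when airborne.
; A counter-force damps sideways sliding.
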(event EventBeginPlay
  (Physics|SetSimulatePhysics (Variables|Default|GetSphere) true))

(event Collision|EventActorBeginOverlap
  (params (OtherActor :type Actor%20Object%20Reference)))

(event EventTick
  (params (DeltaSeconds :type Float%20%28single-precision%29))
  (|SetSphereRotation)
  (|AlignHoverboard)
  (|SetCurrentSpeeds)
  (|SetMovementForces)
  (|LateralStability))

(event Input|AxisEvents|InputAxisMoveForward
  (params (AxisValue :type Float%20%28single-precision%29))
  ;[1 1 1] Board Movement (WASD)
  (Variables|Default|SetTargetSpeed (* AxisValue 5e+03)))

(event Input|AxisEvents|InputAxisMoveRight
  (params (AxisValue :type Float%20%28single-precision%29))
  ;[1 1 1] Board Movement (WASD)
  (Variables|Default|SetTargetAngularSpeed (* AxisValue 1e+02)))

(event Input|AxisEvents|InputAxisLookUp
  (params (AxisValue :type Float%20%28single-precision%29))
  ;[1 1 1] Mouse Movement (Third Person)
  (Transformation|AddRelativeRotation (Variables|Default|GetBoom) (Math|Rotator|MakeRotator 0.0 (* AxisValue -1.0) 0.0) false false))

(event Input|AxisEvents|InputAxisTurn
  (params (AxisValue :type Float%20%28single-precision%29))
  ;[1 1 1] Mouse Movement (Third Person)
  (Transformation|AddRelativeRotation (Variables|Default|GetBoom) (Math|Rotator|MakeRotator 0.0 0.0 AxisValue) false false))

(fn ConstructionScript)

(fn LineTrace
  (params (InputLocation :type Vector))
  (bind _hoverboard (Variables|Default|GetHoverboard))
  (bind _returnvalue (Math|Vector|GetUpVector _hoverboard))
  (bind _returnvalue_2 (* _returnvalue 2e+02))
  (bind _returnvalue_3 (- InputLocation _returnvalue_2))
  (bind (_outhit _returnvalue_4) (Collision|LineTraceByChannel InputLocation _returnvalue_3 "TraceTypeQuery2" false 0 "ForOneFrame"))
  (if _returnvalue_4
    (return (.Location (Collision|BreakHitResult _outhit)) (.Normal (Collision|BreakHitResult _outhit)) true)
    (else
      (return _returnvalue_3 "0,0,1.000000" false))))

(fn GetSimulatedVelocity
  (bind _returnvalue (Physics|GetPhysicsLinearVelocity (Variables|Default|GetSphere) "None"))
  (return _returnvalue (Math|Vector|VectorLength _returnvalue)))

(fn DetermineGrounded
  (Variables|Default|SetHoverboardGrounded (Math|Boolean|ANDBoolean (Variables|Default|GetFrontIsHitting) (Variables|Default|GetBackIsHitting) (Variables|Default|GetFLIsHitting) (Variables|Default|GetFRIsHitting)))
  (if (Variables|Default|GetHoverboardGrounded)
    (Variables|Default|SetIsGrounded true :!label _label)
    (else
      (if (Variables|Default|GetHoverboardFlying)
        (if (Math|Boolean|ORBoolean (Variables|Default|GetFRIsHitting) (Variables|Default|GetFLIsHitting) (Variables|Default|GetFrontIsHitting) (Variables|Default|GetBackIsHitting) (Variables|Default|GetSphereHitting))
          (goto _label)
          (else
            _)))
      (Variables|Default|SetIsGrounded false)))
  (Variables|Default|SetHoverboardFlying (Math|Boolean|ANDBoolean (not (Variables|Default|GetFrontIsHitting)) (not (Variables|Default|GetBackIsHitting)) (not (Variables|Default|GetFLIsHitting)) (not (Variables|Default|GetFRIsHitting)) (not (Variables|Default|GetSphereHitting)))))